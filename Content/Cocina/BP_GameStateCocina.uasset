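; Game state Blueprint for a kitchen game that puts the player-facing UI on screen as the match progresses.
; On BeginPlay it creates the HUD widget and adds it to the viewport.
; A match-state change event shows the end-of-match widget when the state reaches its finished value.
; Score and recipe change events only print their new values to screen, with no UI update here.
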(event EventBeginPlay
  (bind _returnvalue (UserInterface|CreateWidget "/Game/Cocina/WBP_HUD.WBP_HUD_C"))
  (UserInterface|Viewport|AddtoViewport _returnvalue 0))

(event EventTick
  (params (DeltaSeconds :type Float%20%28single-precision%29)))

(event EventOnPuntuacionCambio
  (params (NuevaPuntuacion :type Integer))
  (Development|PrintString (Utilities|String|ToString(Integer) NuevaPuntuacion)))

(event EventOnEstadoPartidaCambio
  (params (Nuevo :type EEstadoPartida%20Enum :default "Esperando"))
  (if (== Nuevo 2)
    (bind _returnvalue (UserInterface|CreateWidget "/Game/Cocina/UI/WBP_FinPartida.WBP_FinPartida_C"))
    (UserInterface|Viewport|AddtoViewport _returnvalue 0)))

(event EventOnRecetaCambio
  (params (NuevoIndice :type Integer))
  (Development|PrintString (Utilities|String|ToString(Integer) NuevoIndice)))

(fn ConstructionScript)